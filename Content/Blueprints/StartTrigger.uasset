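; StartTrigger is a touch trigger that opens level selection when the MotionControllerPawn overlaps its Box.
; On play it hides its cube, text and overlap detection, along with the LevelSpheres and their collision; EnableView, not called within this Blueprint, re-arms it.
; A pawn overlap reveals the spheres with collision, disables the trigger again and calls LevelSelectionSeq on Kay.
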(event `self.ReceiveBeginPlay`
  (`self.DisableView`)
  (for _array_element (`self.LevelSpheres`)
    (`self.SetActorHiddenInGame` _array_element true)
    (`self.SetActorEnableCollision` _array_element false)))

(event `self.Box.OnComponentBeginOverlap`
  (params (OverlappedComponent :type "PrimitiveComponent Object Reference") (OtherActor :type "Actor Object Reference") (OtherComp :type "PrimitiveComponent Object Reference") (OtherBodyIndex :type Integer) (bFromSweep :type Boolean) (SweepResult :type "HitResult Structure (by ref)"))
  (cast `/Game/VirtualRealityBP/Blueprints/MotionControllerPawn` OtherActor)
  (for _array_element (`self.LevelSpheres`)
    (`self.SetActorHiddenInGame` _array_element false)
    (`self.SetActorEnableCollision` _array_element true))
  (`self.DisableView`)
  (`/Game/Blueprints/UI/BP_Kay.LevelSelectionSeq` (`self.Kay`)))

(fn `DisableView`
  (`SceneComponent.SetVisibility` (`self.Cube`) false false)
  (`SceneComponent.SetVisibility` (`self.TextRender`) false false)
  (set `PrimitiveComponent.bGenerateOverlapEvents` false (`self.Box`)))

(fn `EnableView`
  (`SceneComponent.SetVisibility` (`self.Cube`) true false)
  (`SceneComponent.SetVisibility` (`self.TextRender`) true false)
  (set `PrimitiveComponent.bGenerateOverlapEvents` true (`self.Box`)))

(fn `UserConstructionScript`)