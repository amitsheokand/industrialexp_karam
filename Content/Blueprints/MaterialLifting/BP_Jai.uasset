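; BP_Jai directs a material-lifting training scenario for a motion-controller pawn, timing voice-over, info screens and level sequences with chained Delays.
; The externally triggered welcome leads to knot-selection plates, which call back through MrKnot to play each knot's video.
; Plates return when a video ends; Close hides them.
; Separate events handle the drop point, fall audio and player reset, though several are only Delay stubs and hook setup is disconnected.
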(event `self.ReceiveBeginPlay`
  (`self.Initailze`)
  (bind _asmotion_controller_pawn (cast `/Game/VirtualRealityBP/Blueprints/MotionControllerPawn` (`GameplayStatics.GetPlayerPawn` 0)))
  (set `self.Player` _asmotion_controller_pawn))

(event `EventWelcome`
  (`self.IntroSequence`)
  (`KismetSystemLibrary.Delay` 14.0)
  (`self.EventKnotMessage`))

(event `EventKnotMessage`
  (`self.SelectKnotsMessage`)
  (`KismetSystemLibrary.Delay` 9.0)
  (`self.SetMessageScreen` false)
  (`self.EnableKnots`))

(event `AfterKnotsMessage`
  (`KismetSystemLibrary.Delay` 3.0))

(event `EventSimulateRadhe`
  (`KismetSystemLibrary.Delay` 12.0))

(event `OnPlayerReachDropPoint`
  (`MovieSceneSequencePlayer.Play` (`LevelSequenceActor.SequencePlayer` (`self.BirdSequence`)))
  (`self.SetActorEnableCollision` (`self.FallStopper`) true)
  (`KismetSystemLibrary.Delay` 1.5))

(event `ResumeAfterFall`
  (params (delayAmount :type "Float (double-precision)"))
  (`KismetSystemLibrary.Delay` delayAmount))

(event `ResetPlayerAfterFall`
  (`self.K2_SetActorLocation` (`GameplayStatics.GetPlayerPawn` 0) (2548.0 1344.0 11.0) false false)
  (bind _asmotion_controller_pawn (cast `/Game/VirtualRealityBP/Blueprints/MotionControllerPawn` (`GameplayStatics.GetPlayerPawn` 0)))
  (`/Game/VirtualRealityBP/Blueprints/MotionControllerPawn.DisableMIcron` _asmotion_controller_pawn)
  (`self.HidePlayerHooks`)
  (`self.ResumeAfterFall` 15.0))

(event `RenableLanyardChocies`
  (params (delayAmount :type "Float (double-precision)"))
  (`KismetSystemLibrary.Delay` delayAmount))

(event `AfterDisplayMicronFuture`
  (params (delayAmount :type "Float (double-precision)"))
  (`KismetSystemLibrary.Delay` delayAmount)
  (`self.RadheSeq1`))

(event `RadheSeq1`
  (`MovieSceneSequencePlayer.Play` (`LevelSequenceActor.SequencePlayer` (`self.MainSeq`)))
  (`KismetSystemLibrary.Delay` 25.0))

(event `AfterChoosingMicron`
  (`KismetSystemLibrary.Delay` 29.0)
  (`/Game/Blueprints/BP_SoundController.PlaySound` (`self.SoundController`) "/Game/Sounds/TelecomTower/05_-_Protective_Gear.05_-_Protective_Gear"))

(event `DuringFall`
  (`KismetSystemLibrary.Delay` 3.0)
  (`/Game/Blueprints/BP_SoundController.PlaySound` (`self.SoundController`) "/Game/Sounds/PlayerFall-Micron.PlayerFall-Micron")
  (`KismetSystemLibrary.Delay` 10.0)
  (`self.ResetPlayerAfterFall`))

(fn `DisableKnots`
  (for _array_element (`self.KnotsSelectPlates`)
    (`/Game/Blueprints/Telecom/BP_SelectionPlate.HidePlate` _array_element))
  (`/Game/Blueprints/Telecom/BP_ClosePlate.HidePlate` (`self.KnotsClose`)))

(fn `EnableKnots`
  (for _array_element (`self.KnotsSelectPlates`)
    (`/Game/Blueprints/Telecom/BP_SelectionPlate.ShowPlate` _array_element))
  (`/Game/Blueprints/Telecom/BP_ClosePlate.ShowPlate` (`self.KnotsClose`)))

(fn `HidePlayerHooks`
  (`self.SetActorHiddenInGame` (`self.hook1`) true)
  (`self.SetActorHiddenInGame` (`self.hook2`) true))

(fn `Initailze`
  (`|ExecutionSequence`
    (:`then_0`
      (bind _returnvalue (`GameplayStatics.GetActorOfClass` "/Game/Blueprints/BP_SoundController.BP_SoundController_C"))
      (set `self.SoundController` _returnvalue)
      (bind _aswb_material_lifting (cast `/Game/Blueprints/UI/WB_MaterialLifting` (`WidgetComponent.GetUserWidgetObject` (`self.UiWidget`))))
      (set `self.InfoWidget` _aswb_material_lifting)
      (for _array_element (`self.KnotsSelectPlates`)
        (set `/Game/Blueprints/Telecom/BP_SelectionPlate.MrKnot` self _array_element))
      (`self.DisableKnots`)
      (`MediaPlayer.SetLooping` (`self.MediaPlayer`) false)
      (`self.SetMessageScreen` false)
      (set `/Game/Blueprints/Telecom/BP_ClosePlate.MrKnot` self (`self.KnotsClose`)))))

(fn `IntroSequence`
  (`/Game/Blueprints/BP_SoundController.PlaySound` (`self.SoundController`) "/Game/Sounds/MaterialLifting/01Welcome.01Welcome")
  (`/Game/Blueprints/UI/WB_MaterialLifting.WelcomeMaterialIntro` (`self.InfoWidget`))
  (`self.SetMessageScreen` true))

(fn `KnotSelected`
  (params (knotName :type String))
  (`SceneComponent.SetVisibility` (`self.BGMesh`) false false)
  (`SceneComponent.SetVisibility` (`self.UiWidget`) false false)
  (`SceneComponent.SetVisibility` (`self.VideoPlane`) true false)
  (for _array_element (`self.KnotsSelectPlates`)
    (`/Game/Blueprints/Telecom/BP_SelectionPlate.HidePlate` _array_element))
  (switch `string` knotName
    (:`Barrel Hitch`
      (`MediaPlayer.OpenSource` (`self.MediaPlayer`) "/Game/Movies/MS_Barrel-Hitch.MS_Barrel-Hitch")
      (add `MediaPlayer.OnEndReached` (`self.MediaPlayer`) (`|CreateDelegate` :!event `OnMovieFinished`) :!label _label))
    (:`Bowline`
      (`MediaPlayer.OpenSource` (`self.MediaPlayer`) "/Game/Movies/MS_Bowline.MS_Bowline")
      (goto _label))
    (:`Clover Hitch`
      (`MediaPlayer.OpenSource` (`self.MediaPlayer`) "/Game/Movies/MS_Clover_hitch.MS_Clover_hitch")
      (goto _label))
    (:`EStar Stopper`
      (`MediaPlayer.OpenSource` (`self.MediaPlayer`) "/Game/Movies/MS-EStar-Stopper.MS-EStar-Stopper")
      (goto _label))
    (:`Figure-8`
      (`MediaPlayer.OpenSource` (`self.MediaPlayer`) "/Game/Movies/MS_Figure-8.MS_Figure-8")
      (goto _label))
    (:`Half Hitch`
      (`MediaPlayer.OpenSource` (`self.MediaPlayer`) "/Game/Movies/MS_Half-Hitch.MS_Half-Hitch")
      (goto _label))
    (:`Klem Heist`
      (`MediaPlayer.OpenSource` (`self.MediaPlayer`) "/Game/Movies/MS_Klemhiest.MS_Klemhiest")
      (goto _label))
    (:`Close`
      (`self.DisableKnots`))))

(fn `OnMovieFinished`
  (`self.EnableKnots`)
  (`SceneComponent.SetVisibility` (`self.VideoPlane`) false false))

(fn `SelectKnotsMessage`
  (`/Game/Blueprints/BP_SoundController.PlaySound` (`self.SoundController`) "/Game/Sounds/MaterialLifting/02SelectKnots.02SelectKnots")
  (`/Game/Blueprints/UI/WB_MaterialLifting.SelectKnots` (`self.InfoWidget`)))

(fn `SetMessageScreen`
  (params (newVisibility :type Boolean))
  (`SceneComponent.SetVisibility` (`self.UiWidget`) newVisibility true)
  (`SceneComponent.SetVisibility` (`self.BGMesh`) newVisibility true))

(fn `SetupHooks`
  (bind _asmotion_controller_pawn (cast `/Game/VirtualRealityBP/Blueprints/MotionControllerPawn` (`GameplayStatics.GetPlayerPawn` 0)))
  (`/Game/VirtualRealityBP/Blueprints/MotionControllerPawn.SetHooks` _asmotion_controller_pawn (`self.hook1`) (`self.hook2`)))

(fn `ShowPlayerHooks`
  (`self.SetActorHiddenInGame` (`self.hook1`) false)
  (`self.SetActorHiddenInGame` (`self.hook2`) false))

(fn `UserConstructionScript`)