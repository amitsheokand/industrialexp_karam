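; BP_ClosePlate is a Telecom plate actor with a tooltip labelled from its Close value, which it passes to MrKnot.KnotSelected when OnClick is called.
; Helper functions toggle the tooltip, and show or hide the plate's mesh together with its collision.
; BeginPlay stores the starting transform, but the grab, drop-return and PlayerHead-overlap logic that calls BP_Kay_Telecom is disconnected, leaving those events empty.
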(event `self.ReceiveBeginPlay`
  (set `self.InitailPos` (`self.K2_GetActorLocation`))
  (set `self.initalRot` (`self.K2_GetActorRotation`))
  (`TextRenderComponent.K2_SetText` (`self.Tooltip`) (`KismetTextLibrary.Conv_StringToText` (`self.Close`))))

(event `self.ReceiveTick`
  (params (DeltaSeconds :type "Float (single-precision)")))

(event `/Game/VirtualRealityBP/Blueprints/PickupActorInterface.Drop`)

(event `/Game/VirtualRealityBP/Blueprints/PickupActorInterface.Pickup`
  (params (AttachTo :type "SceneComponent Object Reference")))

(event `self.StaticMeshComponent.OnComponentBeginOverlap`
  (params (OverlappedComponent :type "PrimitiveComponent Object Reference") (OtherActor :type "Actor Object Reference") (OtherComp :type "PrimitiveComponent Object Reference") (OtherBodyIndex :type Integer) (bFromSweep :type Boolean) (SweepResult :type "HitResult Structure (by ref)")))

(fn `HidePlate`
  (`SceneComponent.SetVisibility` (`self.StaticMeshComponent`) false true)
  (`self.SetActorEnableCollision` false))

(fn `HideTooltip`
  (`SceneComponent.SetVisibility` (`self.Tooltip`) false false))

(fn `OnClick`
  (`/Game/Blueprints/MaterialLifting/BP_Jai.KnotSelected` (`self.MrKnot`) (`self.Close`)))

(fn `ShowPlate`
  (`SceneComponent.SetVisibility` (`self.StaticMeshComponent`) true true)
  (`self.SetActorEnableCollision` true))

(fn `ShowTooltip`
  (`SceneComponent.SetVisibility` (`self.Tooltip`) true false))

(fn `UserConstructionScript`
  (`TextRenderComponent.K2_SetText` (`self.Tooltip`) (`KismetTextLibrary.Conv_StringToText` (`self.Close`))))