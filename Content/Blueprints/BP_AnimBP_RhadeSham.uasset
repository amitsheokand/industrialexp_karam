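; Actor Blueprint for the RhadeSham figure that carries a Micron lanyard rig of cables and hook meshes.
; BeginPlay hides the rig meshes and cable attach point, while the construction script ties MicronCable's end to the second hook mesh.
; SetLanyard attaches two cables to hook point actors, and ReleaseLanyard clears those ends and reattaches that hook mesh to the skeletal mesh.
; Kill is an empty stub.
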(event `self.ReceiveBeginPlay`
  (`SceneComponent.SetHiddenInGame` (`self.SM_PN351`) true true)
  (`SceneComponent.SetHiddenInGame` (`self.Micron`) true true)
  (`SceneComponent.SetHiddenInGame` (`self.CableAttachPoint`) true true)
  (`SceneComponent.SetHiddenInGame` (`self.SM_PN_42_Micron_SM_PN_42_Hook2`) true true)
  (`SceneComponent.SetHiddenInGame` (`self.SM_PN_42_Micron_SM_PN_42_Mid`) true true)
  (`SceneComponent.SetHiddenInGame` (`self.SM_PN_42_Micron_SM_PN_42_Hook1`) true true))

(event `Kill`)

(event `SetLanyard`
  (params (NewState :type Boolean))
  (`CableComponent.SetAttachEndTo` (`self.Cable1`) (`self.HooKPoint`) "None" "None")
  (`CableComponent.SetAttachEndTo` (`self.Cable2`) (`self.HooKPoint2`) "None" "None"))

(event `ReleaseLanyard`
  (`CableComponent.SetAttachEndTo` (`self.Cable1`) null "None" "None")
  (`CableComponent.SetAttachEndTo` (`self.Cable2`) null "None" "None")
  (`SceneComponent.K2_AttachToComponent` (`self.SM_PN_42_Micron_SM_PN_42_Hook2`) (`self.SkeletalMeshComponent`) "None" "KeepRelative" "KeepRelative" "KeepRelative" true))

(fn `UserConstructionScript`
  (`CableComponent.SetAttachEndToComponent` (`self.MicronCable`) (`self.SM_PN_42_Micron_SM_PN_42_Hook2`) "None"))