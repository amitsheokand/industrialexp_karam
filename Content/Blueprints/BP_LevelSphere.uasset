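; Grabbable level-select sphere that loads its named level when brought to the player's head.
; Pickup attaches it to the supplied component and hides its line and text label; Drop detaches it, shows them again and moves the mesh back toward the saved start transform.
; While grabbable, overlapping a component tagged PlayerHead passes LevelName to BP_MapLoader.
; The actor starts hidden in game.
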(event `self.ReceiveBeginPlay`
  (set `self.InitailPos` (`self.K2_GetActorLocation`))
  (set `self.initalRot` (`self.K2_GetActorRotation`))
  (`self.SetActorHiddenInGame` true))

(event `self.ReceiveTick`
  (params (DeltaSeconds :type "Float (single-precision)")))

(event `/Game/VirtualRealityBP/Blueprints/PickupActorInterface.Drop`
  (if (`self.Grabable`)
    (`self.K2_DetachFromActor` "KeepWorld" "KeepWorld" "KeepWorld")
    (`KismetSystemLibrary.MoveComponentTo` (`self.StaticMeshComponent`) (`self.InitailPos`) (`self.initalRot`) false false 0.2 true)
    (`SceneComponent.SetVisibility` (`self.Line`) true false)
    (`SceneComponent.SetVisibility` (`self.TextRender`) true false)))

(event `/Game/VirtualRealityBP/Blueprints/PickupActorInterface.Pickup`
  (params (AttachTo :type "SceneComponent Object Reference"))
  (if (`self.Grabable`)
    (`SceneComponent.K2_AttachToComponent` (`self.K2_GetRootComponent`) AttachTo "None" "KeepWorld" "KeepWorld" "KeepWorld" false)
    (`SceneComponent.SetVisibility` (`self.Line`) false false)
    (`SceneComponent.SetVisibility` (`self.TextRender`) false false)))

(event `self.StaticMeshComponent.OnComponentBeginOverlap`
  (params (OverlappedComponent :type "PrimitiveComponent Object Reference") (OtherActor :type "Actor Object Reference") (OtherComp :type "PrimitiveComponent Object Reference") (OtherBodyIndex :type Integer) (bFromSweep :type Boolean) (SweepResult :type "HitResult Structure (by ref)"))
  (if (`self.Grabable`)
    (if (`KismetStringLibrary.EqualEqual_StrStr` (`KismetStringLibrary.Conv_NameToString` (`|GetArrayItem` (`ActorComponent.ComponentTags` OtherComp))) "PlayerHead")
      (bind _returnvalue (`GameplayStatics.GetActorOfClass` "/Game/Blueprints/BP_MapLoader.BP_MapLoader_C"))
      (`/Game/Blueprints/BP_MapLoader.On Level Load` _returnvalue (`self.LevelName`)))))

(fn `UserConstructionScript`)