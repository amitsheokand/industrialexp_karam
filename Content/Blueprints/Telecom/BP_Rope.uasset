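; BP_Rope is a telecom rope actor whose cable end can be attached to the VR MotionControllerPawn or handed off to another actor.
; AttachRope caches the player pawn, attaches the CableComponent end to it, sets the cable length and enables following.
; While following, Tick reattaches the cable each frame and copies the pawn's AttachPoint relative location into its end location.
; DettachRope stops following and attaches the end to the given actor.
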(event `self.ReceiveTick`
  (params (DeltaSeconds :type "Float (single-precision)"))
  (bind _player (`self.player`))
  (if (`self.followPlayer`)
    (`CableComponent.SetAttachEndTo` (`self.CableComponent`) _player "None" "None")
    (set `CableComponent.EndLocation` (`SceneComponent.RelativeLocation` (`/Game/VirtualRealityBP/Blueprints/MotionControllerPawn.AttachPoint` _player)) (`self.CableComponent`))))

(fn `AttachRope`
  (bind _cablecomponent (`self.CableComponent`))
  (set `self.followPlayer` true)
  (bind _asmotion_controller_pawn (cast `/Game/VirtualRealityBP/Blueprints/MotionControllerPawn` (`GameplayStatics.GetPlayerPawn` 0)))
  (bind _output_get (set `self.player` _asmotion_controller_pawn))
  (`CableComponent.SetAttachEndTo` _cablecomponent _output_get "None" "None")
  (set `CableComponent.CableLength` 500.0 _cablecomponent))

(fn `DettachRope`
  (params (detachActor :type "Actor Object Reference"))
  (set `self.followPlayer` false)
  (`CableComponent.SetAttachEndTo` (`self.CableComponent`) detachActor "None" "None"))

(fn `UserConstructionScript`)