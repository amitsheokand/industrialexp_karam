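; Scenario controller for telecom-tower fall-hazard training with a motion-controller pawn, guiding PPE and activity choices through sound and a tower widget.
; ChooseOption routes named picks: Micron equips the pawn and opens the ladder, PN9000 re-prompts, Simulate plays RadheSham's climb-and-fall sequence, Perform enables climbing.
; PlayerFall checks the harness, zeroing gravity for safe falls, then after a delay restores gravity, detaches the rope and reopens PPE selection.
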(event `self.ReceiveBeginPlay`
  (`self.Initailze`))

(event `ReEnablePPE`
  (`KismetSystemLibrary.Delay` 4.0)
  (`self.EnableChoosePPE`))

(event `ReEnableSenarios`
  (`KismetSystemLibrary.Delay` 34.0)
  (`self.EnableChoosePPE`)
  (`/Game/Blueprints/Telecom/BP_Rope.DettachRope` (`self.Rope`) null)
  (bind _asmotion_controller_pawn (cast `/Game/VirtualRealityBP/Blueprints/MotionControllerPawn` (`GameplayStatics.GetPlayerPawn` 0)))
  (set `/Game/VirtualRealityBP/Blueprints/MotionControllerPawn.Gravity` 981.0 _asmotion_controller_pawn))

(event `EventSimulateRadhe`
  (`KismetSystemLibrary.Delay` 12.0)
  (`self.EnableChooseActivity`)
  (`KismetSystemLibrary.Delay` 2.0)
  (`self.K2_SetActorLocation` (`self.RadheSham`) (`self.RadheLocation`) false false)
  (`self.K2_SetActorRotation` (`self.RadheSham`) (`self.RoadheRotation`) false))

(event `FallWithMicron`
  (bind _asmotion_controller_pawn (cast `/Game/VirtualRealityBP/Blueprints/MotionControllerPawn` (`GameplayStatics.GetPlayerPawn` 0)))
  (set `/Game/VirtualRealityBP/Blueprints/MotionControllerPawn.Gravity` 0.0 _asmotion_controller_pawn))

(fn `ChooseOption`
  (params (functionName :type String))
  (switch `string` functionName
    (:`Micron`
      (`self.OnMicron`))
    (:`PN9000`
      (`self.OnPN9000`))
    (:`Simulate`
      (`self.OnSimulateActivity`))
    (:`Perform`
      (`self.OnPerformActivity`))))

(fn `DisableChooseActivity`
  (for _array_element (`self.ActivityActors`)
    (`self.SetActorHiddenInGame` _array_element true)
    (`self.SetActorEnableCollision` _array_element false)))

(fn `DisableChoosePPE`
  (for _array_element (`self.PPEActors`)
    (`self.SetActorHiddenInGame` _array_element true)
    (`self.SetActorEnableCollision` _array_element false)))

(fn `DisableLadder`
  (for _array_element (`self.LadderParts`)
    (`self.SetActorEnableCollision` _array_element false)))

(fn `EnableChooseActivity`
  (for _array_element (`self.ActivityActors`)
    (`self.SetActorHiddenInGame` _array_element false)
    (`self.SetActorEnableCollision` _array_element true))
  (`/Game/Blueprints/BP_SoundController.PlaySound` (`self.SoundController`) "/Game/Sounds/00_-_Sim_or_perform.00_-_Sim_or_perform")
  (`/Game/Blueprints/UI/WB_TelecomTower.OnChooseActivity` (`self.InfoWidget`)))

(fn `EnableChoosePPE`
  (for _array_element (`self.PPEActors`)
    (`self.SetActorHiddenInGame` _array_element false)
    (`self.SetActorEnableCollision` _array_element true))
  (`/Game/Blueprints/BP_SoundController.PlaySound` (`self.SoundController`) "/Game/Sounds/04_-_Ask-to-choose.04_-_Ask-to-choose")
  (`/Game/Blueprints/UI/WB_TelecomTower.ChoosePPE` (`self.InfoWidget`)))

(fn `EnableLadder`
  (for _array_element (`self.LadderParts`)
    (`self.SetActorEnableCollision` _array_element true)))

(fn `Initailze`
  (bind _radhesham (`self.RadheSham`))
  (`|ExecutionSequence`
    (:`then_0`
      (bind _returnvalue (`GameplayStatics.GetActorOfClass` "/Game/Blueprints/BP_SoundController.BP_SoundController_C"))
      (set `self.SoundController` _returnvalue)
      (`self.DisableChoosePPE`)
      (`self.DisableChooseActivity`)
      (bind _aswb_telecom_tower (cast `/Game/Blueprints/UI/WB_TelecomTower` (`WidgetComponent.GetUserWidgetObject` (`self.UiWidget`))))
      (set `self.InfoWidget` _aswb_telecom_tower)
      (`self.IntoSequence`)
      (`self.DisableLadder`))
    (:`then_1`
      (set `self.RadheLocation` (`self.K2_GetActorLocation` _radhesham))
      (set `self.RoadheRotation` (`self.K2_GetActorRotation` _radhesham)))))

(fn `IntoSequence`
  (`/Game/Blueprints/BP_SoundController.PlaySound` (`self.SoundController`) "/Game/Sounds/03_-_Define-Hazard.03_-_Define-Hazard")
  (`/Game/Blueprints/UI/WB_TelecomTower.TelecomIntro` (`self.InfoWidget`)))

(fn `OnMicron`
  (`self.DisableChoosePPE`)
  (bind _asmotion_controller_pawn (cast `/Game/VirtualRealityBP/Blueprints/MotionControllerPawn` (`GameplayStatics.GetPlayerPawn` 0)))
  (`/Game/VirtualRealityBP/Blueprints/MotionControllerPawn.EnableMicron` _asmotion_controller_pawn)
  (`/Game/Blueprints/BP_SoundController.PlaySound` (`self.SoundController`) "/Game/Sounds/04_2_Choose-Right.04_2_Choose-Right")
  (`/Game/Blueprints/UI/WB_TelecomTower.OnChooseMicron` (`self.InfoWidget`))
  (`PrimitiveComponent.SetCollisionEnabled` (`/Game/Blueprints/Telecom/BP_ClimbTRigger.Box` (`self.RopeTrigger`)) "QueryOnly")
  (`self.EnableLadder`))

(fn `OnPerformActivity`
  (`PrimitiveComponent.SetCollisionEnabled` (`/Game/Blueprints/Telecom/BP_ClimbTRigger.Box` (`self.RopeTrigger`)) "QueryOnly")
  (`self.DisableChooseActivity`)
  (`/Game/Blueprints/BP_SoundController.PlaySound` (`self.SoundController`) "/Game/Sounds/PerformWithoutMicron.PerformWithoutMicron")
  (`self.EnableLadder`)
  (`/Game/Blueprints/UI/WB_TelecomTower.OnChoosePerform` (`self.InfoWidget`)))

(fn `OnPN9000`
  (`self.DisableChoosePPE`)
  (`/Game/Blueprints/BP_SoundController.PlaySound` (`self.SoundController`) "/Game/Sounds/04_1_Choose-wrong.04_1_Choose-wrong")
  (`self.ReEnablePPE`)
  (`/Game/Blueprints/UI/WB_TelecomTower.OnChoosePN4000` (`self.InfoWidget`)))

(fn `OnSimulateActivity`
  (bind _radhesham (`self.RadheSham`))
  (`/Game/Blueprints/BP_SoundController.PlaySound` (`self.SoundController`) "/Game/Sounds/Simulate.Simulate")
  (`self.SetActorHiddenInGame` _radhesham false)
  (`self.SetActorEnableCollision` _radhesham true)
  (`self.DisableChooseActivity`)
  (`MovieSceneSequencePlayer.Play` (`LevelSequenceActor.SequencePlayer` (`self.ClimbnFall`)))
  (`/Game/Blueprints/UI/WB_TelecomTower.OnChooseSimulate` (`self.InfoWidget`))
  (`self.EventSimulateRadhe`))

(fn `PlayerFall`
  (bind _soundcontroller (`self.SoundController`))
  (`self.DisableLadder`)
  (bind _asmotion_controller_pawn (cast `/Game/VirtualRealityBP/Blueprints/MotionControllerPawn` (`GameplayStatics.GetPlayerPawn` 0)))
  (if (`/Game/VirtualRealityBP/Blueprints/MotionControllerPawn.HasHarness` _asmotion_controller_pawn)
    (`/Game/Blueprints/BP_SoundController.PlaySound` _soundcontroller "/Game/Sounds/10_-_Safe-Fall.10_-_Safe-Fall")
    (`self.FallWithMicron`)
    (`/Game/Blueprints/UI/WB_TelecomTower.FallSafe` (`self.InfoWidget`))
    (else
      (`/Game/Blueprints/BP_SoundController.PlaySound` _soundcontroller "/Game/Sounds/OnFall.OnFall")
      (`/Game/Blueprints/UI/WB_TelecomTower.FallUnsafe` (`self.InfoWidget`))))
  (`self.ReEnableSenarios`))

(fn `UserConstructionScript`)