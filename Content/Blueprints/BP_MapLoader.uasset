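; Map loader actor that swaps streamed levels at runtime, starting with LevelSelection on BeginPlay.
; OnLevelLoad unloads the current LoadedLevel, then creates a uniquely named streaming level instance from an incrementing index, makes it loaded and visible, and stores it.
; ResetPlayer then moves the player pawn to a hardcoded location, defined only for the Karam level, without waiting for the load to finish.
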(event `self.ReceiveBeginPlay`
  (`self.On Level Load` "LevelSelection"))

(fn `On Level Load`
  (params (levelName :type String))
  (`self.OnLevelUnload`)
  (set `self.instanceIndex` (+ (`self.instanceIndex`) 1))
  (bind _returnvalue (`LevelStreaming.CreateInstance` (`GameplayStatics.GetStreamingLevel` (`KismetStringLibrary.Conv_StringToName` levelName)) (`KismetStringLibrary.Conv_IntToString` (`self.instanceIndex`))))
  (set `LevelStreaming.bShouldBeLoaded` true _returnvalue)
  (set `LevelStreaming.bShouldBeVisible` true _returnvalue)
  (set `self.LoadedLevel` _returnvalue)
  (`self.ResetPlayer` levelName))

(fn `OnLevelUnload`
  (if (!= (`self.LoadedLevel`) null)
    (set `LevelStreaming.bShouldBeLoaded` false (`self.LoadedLevel`))))

(fn `ResetPlayer`
  (params (lvlName :type String))
  (switch `string` lvlName
    (:`karam`
      (`self.K2_SetActorLocation` (`GameplayStatics.GetPlayerPawn` 0) (2548.0 1344.0 11.0) false false))))

(fn `UserConstructionScript`)